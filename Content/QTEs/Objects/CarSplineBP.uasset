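; CarSplineBP is a car obstacle, filed under QTE objects, that drives along a spline and ragdolls the player character on overlap.
; Tick advances distance by SplineSpeed and snaps the Car's relative transform to the spline's local transform with a fixed downward offset, restarting at the end if Loop is set.
; Overlapping a QTECharacter02 calls its Ragdoll, and clicking the actor stops the car by zeroing its speed.
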(event `self.ReceiveTick`
  (params (DeltaSeconds :type "Float (single-precision)"))
  (bind _returnvalue (`SplineComponent.GetTransformAtDistanceAlongSpline` (`self.Spline`) (`self.Distance Alone Spline`) "Local" false))
  ;[1 1 1] Spline/Movement
  (set `self.Distance Alone Spline` (+ (* DeltaSeconds (`self.SplineSpeed`)) (`self.Distance Alone Spline`)))
  (`SceneComponent.K2_SetRelativeTransform` (`self.Car`) (`KismetMathLibrary.MakeTransform` (`KismetMathLibrary.MakeVector` (.x (.location _returnvalue)) (.y (.location _returnvalue)) (+ (.z (.location _returnvalue)) -89.0)) (`KismetMathLibrary.MakeRotator` (.roll (.rotation _returnvalue)) (.pitch (.rotation _returnvalue)) (.yaw (.rotation _returnvalue)))) false false)
  (if (`self.Loop?`)
    (if (> (`self.Distance Alone Spline`) (`SplineComponent.GetSplineLength` (`self.Spline`)))
      (set `self.Distance Alone Spline` 0.0))))

(event `self.ReceiveActorBeginOverlap`
  (params (OtherActor :type "Actor Object Reference"))
  ;[1 1 1] Ragdoll Player on Collision
  (bind _asqtecharacter_02 (cast `/Game/ThirdPerson/Blueprints/QTECharacter02` OtherActor))
  (`/Game/ThirdPerson/Blueprints/QTECharacter02.Ragdoll` _asqtecharacter_02))

(event `self.ReceiveActorOnClicked`
  (params (ButtonPressed :type "Key Structure"))
  ;[1 1 1] Stop Movement
  (set `self.SplineSpeed` 0.0))

(fn `UserConstructionScript`)