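; Spline actor in the QTE objects folder that moves its Plane component along its spline at a set speed.
; Each Tick advances a distance by SplineSpeed and DeltaSeconds, then copies the local spline location and rotation to the Plane, with a fixed downward Z offset.
; When Loop is enabled, the distance resets to zero once it exceeds the spline length.
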(event `self.ReceiveTick`
  (params (DeltaSeconds :type "Float (single-precision)"))
  (bind _returnvalue (`SplineComponent.GetTransformAtDistanceAlongSpline` (`self.Spline`) (`self.Distance Alone Spline`) "Local" false))
  (set `self.Distance Alone Spline` (+ (* DeltaSeconds (`self.SplineSpeed`)) (`self.Distance Alone Spline`)))
  (`SceneComponent.K2_SetRelativeTransform` (`self.Plane`) (`KismetMathLibrary.MakeTransform` (`KismetMathLibrary.MakeVector` (.x (.location _returnvalue)) (.y (.location _returnvalue)) (+ (.z (.location _returnvalue)) -89.0)) (`KismetMathLibrary.MakeRotator` (.roll (.rotation _returnvalue)) (.pitch (.rotation _returnvalue)) (.yaw (.rotation _returnvalue)))) false false)
  (if (`self.Loop?`)
    (if (> (`self.Distance Alone Spline`) (`SplineComponent.GetSplineLength` (`self.Spline`)))
      (set `self.Distance Alone Spline` 0.0))))

(fn `UserConstructionScript`)