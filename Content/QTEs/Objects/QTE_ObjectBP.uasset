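; QTE obstacle actor with a clickable manhole mesh and a trigger box that ragdolls any QTECharacter that overlaps it.
; Clicking drives the Moving timeline, which lerps the manhole's relative location between the origin and EndLocation.
; The Clicked flag selects reverse or play, but each branch writes back the value it tested, so clicks never toggle the direction.
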(event `self.Box.OnComponentBeginOverlap`
  (params (OverlappedComponent :type "PrimitiveComponent Object Reference") (OtherActor :type "Actor Object Reference") (OtherComp :type "PrimitiveComponent Object Reference") (OtherBodyIndex :type Integer) (bFromSweep :type Boolean) (SweepResult :type "HitResult Structure (by ref)"))
  (bind _asqtecharacter (cast `/Game/ThirdPerson/Blueprints/QTECharacter` OtherActor))
  (`/Game/ThirdPerson/Blueprints/QTECharacter.Ragdoll` _asqtecharacter))

(event `self.ReceiveActorOnClicked`
  (params (ButtonPressed :type "Key Structure"))
  (if (`self.Clicked?`)
    (set `self.Clicked?` true)
    (bind (_direction _movement) (`Timeline|Moving` :!via `Reverse` :!label _label)
      (:`Update`
        (`SceneComponent.K2_SetRelativeLocation` (`self.Manhole`) (`KismetMathLibrary.VLerp` (0.0 0.0 0.0) (`self.End Location`) _movement) false false)))
    (else
      (set `self.Clicked?` false)
      (goto _label))))

(fn `UserConstructionScript`)